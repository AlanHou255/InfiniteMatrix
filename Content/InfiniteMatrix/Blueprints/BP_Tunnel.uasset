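; BP_Tunnel is an endless-runner tunnel segment with a rotating holed wall as the obstacle.
; RandomizeWall picks one of four hole meshes and a random roll, and Tick keeps it spinning.
; A player entering TriggerZone makes TunnelSpawner add a segment and randomly spawn an enemy or health pack ahead, scores a point, and destroys this segment.
; Wall hits cost health and score or trigger restart at zero health, and destroy projectiles.
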(event OnComponentBeginOverlap(TriggerZone)
  (params (OverlappedComponent :type Primitive%20Component%20Object%20Reference) (OtherActor :type Actor%20Object%20Reference) (OtherComp :type Primitive%20Component%20Object%20Reference) (OtherBodyIndex :type Integer) (bFromSweep :type Boolean) (SweepResult :type Hit%20Result%20Structure%20%28by%20ref%29))
  (bind _returnvalue (Math|Random|RandomFloatinRange -2.5e+02 2.5e+02))
  (bind _returnvalue_2 (Math|Random|RandomFloatinRange -2.5e+02 2.5e+02))
  (bind _returnvalue_3 (Game|Player|GetPlayerPawn 0))
  (bind _tunnelspawner (Variables|Default|GetTunnelSpawner))
  (bind _returnvalue_4 (Transformation|GetActorLocation _returnvalue_3))
  (bind _returnvalue_5 (+ (.x _returnvalue_4) 7.25e+03))
  (bind _returnvalue_6 (+ (.x _returnvalue_4) 5.25e+03))
  (bind _returnvalue_7 (Math|Random|RandomFloatinRange _returnvalue_6 _returnvalue_5))
  (bind _asbp_player (Utilities|Casting|CastToBP_Player OtherActor))
  (Default|SpawnTunnelatSpawnPoint (Variables|Default|GetTunnelSpawner))
  (Actor|DestroyActor)
  (Variables|/Game/InfiniteMatrix/Blueprints/BP_Player.BP_Player_C|SetScore _asbp_player (+ (Variables|/Game/InfiniteMatrix/Blueprints/BP_Player.BP_Player_C|GetScore _asbp_player) 1))
  (if (> (Math|Random|RandomFloat) 0.79)
    (Default|SpawnHealthPack _tunnelspawner (Math|Vector|MakeVector _returnvalue_7 _returnvalue_2 _returnvalue))
    (else
      (Default|SpawnEnemy _tunnelspawner (Math|Vector|MakeVector _returnvalue_7 _returnvalue_2 _returnvalue)))))

(event OnComponentBeginOverlap(WallMesh)
  (params (OverlappedComponent :type Primitive%20Component%20Object%20Reference) (OtherActor :type Actor%20Object%20Reference) (OtherComp :type Primitive%20Component%20Object%20Reference) (OtherBodyIndex :type Integer) (bFromSweep :type Boolean) (SweepResult :type Hit%20Result%20Structure%20%28by%20ref%29))
  (bind _asbp_player (Utilities|Casting|CastToBP_Player OtherActor)
    (:then
      (bind _output_get (Variables|/Game/InfiniteMatrix/Blueprints/BP_Player.BP_Player_C|SetHealth _asbp_player (- (Variables|/Game/InfiniteMatrix/Blueprints/BP_Player.BP_Player_C|GetHealth _asbp_player) 0.2)))
      (if (<= _output_get 0.01)
        (Default|DisplayRestart _asbp_player)
        (Variables|/Game/InfiniteMatrix/Blueprints/BP_Player.BP_Player_C|SetForwardSpeed _asbp_player 0.0)
        (else
          (Variables|/Game/InfiniteMatrix/Blueprints/BP_Player.BP_Player_C|SetScore _asbp_player (- (Variables|/Game/InfiniteMatrix/Blueprints/BP_Player.BP_Player_C|GetScore _asbp_player) 1))
          (bind _returnvalue (UserInterface|CreateWidget "/Game/InfiniteMatrix/Blueprints/hurtWidget.hurtWidget_C"))
          (UserInterface|Viewport|AddtoViewport _returnvalue 0))))
    (:CastFailed
      (bind _asbp_projectile_player (Utilities|Casting|CastToBP_projectile_player OtherActor)
        (:then
          (Actor|DestroyActor _asbp_projectile_player))
        (:CastFailed
          (bind _asbp_projectile_enemy (Utilities|Casting|CastToBP_projectile_enemy OtherActor))
          (Actor|DestroyActor _asbp_projectile_enemy))))))

(event EventBeginPlay)

(event EventTick
  (params (DeltaSeconds :type Float%20%28single-precision%29))
  (Transformation|AddLocalRotation (Variables|Default|GetWallMesh) (Math|Rotator|MakeRotator (* DeltaSeconds (Variables|Default|GetRotateSpeed)) 0.0 0.0) false false))

(fn ConstructionScript)

(fn RandomizeWall
  (Components|StaticMesh|SetStaticMesh (Variables|Default|GetWallMesh) (Utilities|Select :Index (Math|Random|RandomIntegerinRange 0 3) :Option%200 "/Game/InfiniteMatrix/Meshes/SM_Hole_01.SM_Hole_01" :Option%201 "/Game/InfiniteMatrix/Meshes/SM_Hole_02.SM_Hole_02" :Option%202 "/Game/InfiniteMatrix/Meshes/SM_Hole_03.SM_Hole_03" :Option%203 "/Game/InfiniteMatrix/Meshes/SM_Hole_04.SM_Hole_04"))
  (Transformation|AddLocalRotation (Variables|Default|GetWallMesh) (Math|Rotator|MakeRotator (Math|Random|RandomFloatinRange 0.0 3.6e+02) 0.0 0.0) false false))
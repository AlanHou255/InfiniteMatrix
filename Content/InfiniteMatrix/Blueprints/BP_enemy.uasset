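; BP_enemy is an enemy actor that fires at spawn and damages the player on contact.
; On BeginPlay it spawns a single BP_projectile_enemy at its own location.
; Its Sphere overlap casts to BP_Player and directly reduces Health, adding a HurtWidget to the viewport while health remains.
; When health is depleted, it shows the player's restart display, zeroes ForwardSpeed and destroys itself.
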(event OnComponentBeginOverlap(Sphere)
  (params (OverlappedComponent :type Primitive%20Component%20Object%20Reference) (OtherActor :type Actor%20Object%20Reference) (OtherComp :type Primitive%20Component%20Object%20Reference) (OtherBodyIndex :type Integer) (bFromSweep :type Boolean) (SweepResult :type Hit%20Result%20Structure%20%28by%20ref%29))
  (bind _asbp_player (Utilities|Casting|CastToBP_Player OtherActor))
  (bind _output_get (Variables|/Game/InfiniteMatrix/Blueprints/BP_Player.BP_Player_C|SetHealth _asbp_player (- (Variables|/Game/InfiniteMatrix/Blueprints/BP_Player.BP_Player_C|GetHealth _asbp_player) 0.2)))
  (if (<= _output_get 0.01)
    (Default|DisplayRestart _asbp_player)
    (Variables|/Game/InfiniteMatrix/Blueprints/BP_Player.BP_Player_C|SetForwardSpeed _asbp_player 0.0)
    (Actor|DestroyActor)
    (else
      (bind _returnvalue (UserInterface|CreateWidget "/Game/InfiniteMatrix/Blueprints/hurtWidget.hurtWidget_C"))
      (UserInterface|Viewport|AddtoViewport _returnvalue 0))))

(event EventBeginPlay
  (Game|SpawnActorfromClass "/Game/InfiniteMatrix/Blueprints/BP_projectile_enemy.BP_projectile_enemy_C" (Math|Transform|MakeTransform (Transformation|GetActorLocation) "0, 0, 0" "1,1,1") "Undefined" 0 0))

(event Collision|EventActorBeginOverlap
  (params (OtherActor :type Actor%20Object%20Reference)))

(event EventTick
  (params (DeltaSeconds :type Float%20%28single-precision%29)))

(fn ConstructionScript)